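; Weapon Blueprint that fires projectiles automatically while its trigger is held.
; PullTrigger passes a DoOnce gate to fire immediately, then starts a looping timer paced by RoundPerSecond for repeat shots.
; Fire plays a blast sound attached to the gun mesh and spawns a projectile at ProjectileSpawnPoint.
; ReleaseTrigger clears the Fire timer and resets the gate, so re-pulling shoots instantly with no cooldown.
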(event `PullTrigger`
  (`/Engine/EditorBlueprintResources/StandardMacros.DoOnce` false :!label _label
    (:`Completed`
      (`self.Fire`)
      (`KismetSystemLibrary.K2_SetTimer` null "" (/ 1.0 (`self.RoundPerSecond`)) true))))

(event `ReleaseTrigger`
  (`KismetSystemLibrary.K2_ClearTimer` null "Fire")
  (goto _label :!via `Reset`))

(event `Fire`
  (`GameplayStatics.SpawnSoundAttached` "/Game/Audio/light_blast_6.light_blast_6" (`self.GunMesh`) "None" (0.0 0.0 0.0) (struct) "KeepRelativeOffset" false 1.0 1.0 0.0 null null)
  (`|SpawnActorFromClass` "/Game/Blueprints/Projectile.Projectile_C" (`SceneComponent.K2_GetComponentToWorld` (`self.ProjectileSpawnPoint`)) "Undefined" "MultiplyWithRoot" null null))

(fn `UserConstructionScript`)